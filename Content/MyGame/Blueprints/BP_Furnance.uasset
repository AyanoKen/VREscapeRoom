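; Furnace puzzle actor that consumes BP_Book actors entering its Box trigger and expects their numbers in non-decreasing order.
; Each in-order book updates the current number and count, an out-of-order one permanently sets a fail flag, and every book is destroyed.
; Once ten books count without failure, it prints success, removes the flames and trigger, and slides the referenced wall and furnace using timelines.
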(event OnComponentBeginOverlap(Box)
  (params (OverlappedComponent :type Primitive%20Component%20Object%20Reference) (OtherActor :type Actor%20Object%20Reference) (OtherComp :type Primitive%20Component%20Object%20Reference) (OtherBodyIndex :type Integer) (bFromSweep :type Boolean) (SweepResult :type Hit%20Result%20Structure%20%28by%20ref%29))
  (bind _asbp_book (Utilities|Casting|CastToBP_Book OtherActor))
  (if (>= (Variables|/Game/MyGame/Blueprints/BP_Book.BP_Book_C|GetNumber _asbp_book) (Variables|Default|GetCurrentNumber))
    (Variables|Default|SetCurrentNumber (Variables|/Game/MyGame/Blueprints/BP_Book.BP_Book_C|GetNumber _asbp_book))
    (Variables|Default|SetCount (+ (Variables|Default|GetCount) 1))
    (if (>= (Variables|Default|GetCount) 10)
      (CallFunction|CheckLevelEnd))
    (else
      (Variables|Default|SetFailLevel true)))
  (Actor|DestroyActor _asbp_book))

(event Custom|MoveDoors
  (Variables|Default|SetInitial%20Wall%20Location (Transformation|GetWorldLocation (Variables|/Script/Engine.StaticMeshActor|GetStaticMeshComponent (Variables|Default|GetWall))))
  (bind _wall (Timeline|WallTimeline Play)
    (:Update
      (Transformation|SetWorldLocation (Variables|/Script/Engine.StaticMeshActor|GetStaticMeshComponent (Variables|Default|GetWall)) (Math|Vector|MakeVector (.x (Variables|Default|GetInitial%20Wall%20Location)) (+ _wall (.y (Variables|Default|GetInitial%20Wall%20Location))) (.z (Variables|Default|GetInitial%20Wall%20Location))) false false))))

(event Custom|MoveFurnance
  (Variables|Default|SetInitial%20Furnance%20Location (Transformation|GetWorldLocation (Variables|/Script/Engine.StaticMeshActor|GetStaticMeshComponent (Variables|Default|GetFurnance))))
  (bind _furnancetimeline (Timeline|FurnanceTimeline Play)
    (:Update
      (Transformation|SetWorldLocation (Variables|/Script/Engine.StaticMeshActor|GetStaticMeshComponent (Variables|Default|GetFurnance)) (Math|Vector|MakeVector (+ _furnancetimeline (.x (Variables|Default|GetInitial%20Furnance%20Location))) (.y (Variables|Default|GetInitial%20Furnance%20Location)) (.z (Variables|Default|GetInitial%20Furnance%20Location))) false false))))

(event EventBeginPlay)

(event Collision|EventActorBeginOverlap
  (params (OtherActor :type Actor%20Object%20Reference)))

(event EventTick
  (params (DeltaSeconds :type Float%20%28single-precision%29)))

(fn ConstructionScript)

(fn CheckLevelEnd
  (if (not (Variables|Default|GetFailLevel))
    (Development|PrintString "Success. Proceed to Next level")
    (for _array_element (Variables|Default|GetFlames)
      (Actor|DestroyActor _array_element))
    (CallFunction|MoveDoors)
    (CallFunction|MoveFurnance)
    (Components|DestroyComponent (Variables|Default|GetBox))))