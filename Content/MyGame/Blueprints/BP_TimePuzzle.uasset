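; BP_TimePuzzle is a puzzle that opens a gate once the books numbered 6 and 0 are placed in their slots.
; Each trigger box checks an overlapping BP_Book's number, then removes its grab component, moves it to the Hours or Zero marker, and destroys that marker and box.
; The first placement sets the OpenGate flag; the second plays a timeline that offsets the Cube gate along Z.
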(event OnComponentBeginOverlap(Box)
  (params (OverlappedComponent :type Primitive%20Component%20Object%20Reference) (OtherActor :type Actor%20Object%20Reference) (OtherComp :type Primitive%20Component%20Object%20Reference) (OtherBodyIndex :type Integer) (bFromSweep :type Boolean) (SweepResult :type Hit%20Result%20Structure%20%28by%20ref%29))
  (bind _hours (Variables|Default|GetHours))
  (bind _asbp_book (Utilities|Casting|CastToBP_Book OtherActor))
  (if (== (Variables|/Game/MyGame/Blueprints/BP_Book.BP_Book_C|GetNumber _asbp_book) 6)
    (Components|DestroyComponent (Variables|/Game/MyGame/Blueprints/BP_Book.BP_Book_C|GetGrabComponent _asbp_book))
    (Transformation|SetActorLocation _asbp_book (Transformation|GetWorldLocation _hours) false false)
    (Components|DestroyComponent _hours)
    (Components|DestroyComponent (Variables|Default|GetBox))
    (CallFunction|OpenGate)))

(event OnComponentBeginOverlap(Box1)
  (params (OverlappedComponent :type Primitive%20Component%20Object%20Reference) (OtherActor :type Actor%20Object%20Reference) (OtherComp :type Primitive%20Component%20Object%20Reference) (OtherBodyIndex :type Integer) (bFromSweep :type Boolean) (SweepResult :type Hit%20Result%20Structure%20%28by%20ref%29))
  (bind _zero (Variables|Default|GetZero))
  (bind _asbp_book (Utilities|Casting|CastToBP_Book OtherActor))
  (if (== (Variables|/Game/MyGame/Blueprints/BP_Book.BP_Book_C|GetNumber _asbp_book) 0)
    (Components|DestroyComponent (Variables|/Game/MyGame/Blueprints/BP_Book.BP_Book_C|GetGrabComponent _asbp_book))
    (Transformation|SetActorLocation _asbp_book (Transformation|GetWorldLocation _zero) false false)
    (Components|DestroyComponent _zero)
    (Components|DestroyComponent (Variables|Default|GetBox1))
    (CallFunction|OpenGate)))

(event Custom|OpenGate
  (if (Variables|Default|GetOpenGate?)
    (Variables|Default|SetInitialLocation (Transformation|GetWorldLocation (Variables|Default|GetCube)))
    (bind _gatetrack (Timeline|GateTimeline Play)
      (:Update
        (Transformation|SetWorldLocation (Variables|Default|GetCube) (Math|Vector|MakeVector (.x (Variables|Default|GetInitialLocation)) (.y (Variables|Default|GetInitialLocation)) (+ _gatetrack (.z (Variables|Default|GetInitialLocation)))) false false)))
    (else
      (Variables|Default|SetOpenGate? true))))

(event EventBeginPlay)

(event Collision|EventActorBeginOverlap
  (params (OtherActor :type Actor%20Object%20Reference)))

(event EventTick
  (params (DeltaSeconds :type Float%20%28single-precision%29)))

(fn ConstructionScript)